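; AI soldier character that fires a rifle, takes damage and ragdolls on death.
; Incoming damage goes to BPHealthManager and is reported to AI damage sensing, always crediting player 0 as instigator.
; The health manager's death callback enables mesh physics and unpossesses the BP_AI_Controller.
; The Shot event plays the rifle sound and spawns a configured BP_Bullet from the weapon mesh's muzzle socket.
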(event Custom|Shot
  (bind _skeletalmesh (Variables|Default|GetSkeletalMesh))
  (bind _returnvalue (Transformation|GetSocketTransform _skeletalmesh "MuzzleSocket" "RTS_World"))
  (Audio|PlaySoundatLocation "/Game/Audio/Rifle_Cue.Rifle_Cue" (.location _returnvalue) "0, 0, 0" 1.0 1.0 0.0 0 0 0)
  (Game|SpawnActorfromClass "/Game/Blueprints/BP_Bullet.BP_Bullet_C" (Math|Transform|MakeTransform (.location _returnvalue) (.rotation _returnvalue) "1,1,1") "Undefined" 0 2.0 "/Game/FPS_Weapon_Bundle/Weapons/Meshes/Ammunition/556mm_Bullet.556mm_Bullet" 2e+01 0))

(event Custom|OnDeath_Event_0
  (Physics|SetSimulatePhysics (Variables|Character|GetMesh) true)
  (bind _asbp_ai_controller (Utilities|Casting|CastToBP_AI_Controller (Pawn|GetController)))
  (Pawn|UnPossess _asbp_ai_controller))

(event EventBeginPlay
  (EventDispatchers|AssignOnDeath (Variables|Default|GetBP_HealthManager) (delegate Custom|OnDeath_Event_0)))

(event EventTakeDamage
  (params (Damage :type Float%20%28single-precision%29))
  (Default|TakeDamage (Variables|Default|GetBP_HealthManager) Damage)
  (Class|AISenseDamage|ReportDamageEvent self (Game|GetPlayerCharacter 0) 0.0 "0, 0, 0" "0, 0, 0" "None"))

(fn ConstructionScript)