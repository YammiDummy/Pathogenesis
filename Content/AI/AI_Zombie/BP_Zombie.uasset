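; BP_Zombie is an AI zombie enemy that makes montage-driven melee attacks and can take damage.
; A sphere overlap, gated by IsAbleToAttack, damages actors implementing BPI_Damage and plays a flesh-hit sound.
; Incoming damage feeds BPHealthManager and is reported to AI perception with the player as instigator.
; On death the mesh ragdolls and the controller unpossesses it; a DoOnce blocks repeat attacks until the montage completes.
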(event OnComponentBeginOverlap(Sphere)
  (params (OverlappedComponent :type Primitive%20Component%20Object%20Reference) (OtherActor :type Actor%20Object%20Reference) (OtherComp :type Primitive%20Component%20Object%20Reference) (OtherBodyIndex :type Integer) (bFromSweep :type Boolean) (SweepResult :type Hit%20Result%20Structure%20%28by%20ref%29))
  (if (Variables|Default|GetIsAbleToAttack)
    (if (Utilities|DoesObjectImplementInterface OtherActor "/Game/Interfaces/BPI_Damage.BPI_Damage_C")
      (Class|BPIDamage|TakeDamage(Message) OtherActor 3.0)
      (Audio|PlaySoundatLocation "/Game/Audio/Hit_Flesh_Cue.Hit_Flesh_Cue" (Transformation|GetActorLocation) "0, 0, 0" 1.0 1.0 0.0 0 0 0))))

(event Custom|OnDeath_Event_0
  (Physics|SetSimulatePhysics (Variables|Character|GetMesh) true)
  (Pawn|UnPossess (Pawn|GetController)))

(event Custom|MeleeAttack
  (Utilities|FlowControl|DoOnce false :!label _label
    (:Completed
      (Animation|Montage|PlayMontage (Variables|Character|GetMesh) "/Game/Mixamo/Zombie_Attack_Montage.Zombie_Attack_Montage"
        (:OnCompleted
          (goto _label Reset))))))

(event EventBeginPlay
  (EventDispatchers|AssignOnDeath (Variables|Default|GetBP_HealthManager) (delegate Custom|OnDeath_Event_0)))

(event EventTakeDamage
  (params (Damage :type Float%20%28single-precision%29))
  (Default|TakeDamage (Variables|Default|GetBP_HealthManager) Damage)
  (Class|AISenseDamage|ReportDamageEvent self (Game|GetPlayerCharacter 0) 0.0 "0, 0, 0" "0, 0, 0" "None"))

(fn ConstructionScript)