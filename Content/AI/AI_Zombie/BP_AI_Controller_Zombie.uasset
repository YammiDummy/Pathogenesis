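; AI controller for zombies that starts the BT_Zombie behavior tree and requests the BB_Soldier blackboard on BeginPlay.
; On each target perception update, it prints the attitude toward the actor and writes the sensed state to CanSeePlayer, with no filter on the actor.
; A loop that would store the nearest perceived actor as CurrentTarget is disconnected and never runs.
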(event OnPerceptionUpdated(AIPerception)
  (params (UpdatedActors :type Array%20of%20Actor%20Object%20References)))

(event OnTargetPerceptionUpdated(AIPerception)
  (params (Actor :type Actor%20Object%20Reference) (Stimulus :type AI%20Stimulus%20Structure))
  (Development|PrintString (Utilities|String|EnumtoString (Class|PathogenesisAIController|GetAttitudeTowards Actor)))
  (AI|Components|Blackboard|SetValueasBool (AI|GetBlackboard 0) (Utilities|Name|MakeLiteralName "CanSeePlayer") (.bsuccessfullysensed Stimulus)))

(event EventBeginPlay
  (AI|RunBehaviorTree "/Game/AI/AI_Zombie/BT_Zombie.BT_Zombie")
  (Class|AIController|UseBlackboard "/Game/AI/AI_Soldier/Behavior/BB_Soldier.BB_Soldier"))

(fn ConstructionScript)