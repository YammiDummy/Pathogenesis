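; BP_MagMaster is the base Blueprint for a magazine item in the world, configured from its ItemData.
; Its construction script copies count and item name, then casts the data to Mag to set capacity, ammo type and static mesh.
; The item name feeds BPWidgetComponent, and the PopUp event forwards the given character to that component.
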(event EventBeginPlay)

(event Collision|EventActorBeginOverlap
  (params (OtherActor :type Actor%20Object%20Reference)))

(event EventTick
  (params (DeltaSeconds :type Float%20%28single-precision%29)))

(event EventPopUp
  (params (Character :type Top%20Down%20Character%20Object%20Reference))
  (Default|PopUp (Variables|Default|GetBP_WidgetComponent) Character))

(fn ConstructionScript
  (bind _itemdata (Variables|Default|GetItemData))
  (Variables|Default|SetCount (Variables|/Script/Pathogenesis.Item|GetCount _itemdata))
  (Variables|/Game/Blueprints/Components/BP_WidgetComponent.BP_WidgetComponent_C|SetName (Variables|Default|GetBP_WidgetComponent) (Variables|/Script/Pathogenesis.Item|GetItemName _itemdata))
  (bind _asmag (Utilities|Casting|CastToMag (Variables|Default|GetItemData)))
  (Variables|Default|SetCount (Variables|/Script/Pathogenesis.Item|GetCount _asmag))
  (Variables|Default|SetMaxCapacity (Variables|/Script/Pathogenesis.Mag|GetMagCapacity _asmag))
  (Variables|Default|SetAmmoType (Variables|/Script/Pathogenesis.Mag|GetAmmoType _asmag))
  (Components|StaticMesh|SetStaticMesh (Variables|Default|GetMagMesh) (Variables|/Script/Pathogenesis.Mag|GetMagMesh _asmag)))