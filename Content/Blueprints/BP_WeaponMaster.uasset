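; Base weapon actor that can be picked up and fired, configured from its Weapon item data shortly after BeginPlay.
; Start fires a bullet from the muzzle socket using the current round's stats, with a looping timer for full-auto until Stop clears it.
; Each shot cycles the chamber, ejecting a shell and loading the next round, with a small random jam chance that CleanChamber clears.
; Interact and PopUp handle pickup and the name widget.
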(event EventBeginPlay
  (Utilities|FlowControl|Delay 0.2)
  (CallFunction|Initialize))

(event EventInteract
  (params (Character :type Top%20Down%20Character%20Object%20Reference))
  (Class|PathogenesisCharacter|PickUpItem Character self))

(event EventStart
  (bind _firerate (Variables|Default|GetFireRate))
  (bind _bisfullauto (Variables|Default|GetbIsFullAuto))
  (bind _returnvalue (/ 6e+01 _firerate))
  (if (Variables|Default|GetbIsChamberLoaded)
    (CallFunction|StartFire)
    (if _bisfullauto
      (bind _returnvalue_2 (Utilities|Time|SetTimerbyFunctionName 0 "StartFire" _returnvalue _bisfullauto _returnvalue))
      (Variables|Default|SetFireHandle _returnvalue_2))
    (else
      (Audio|PlaySoundatLocation "/Game/Audio/TriggerClick.TriggerClick" (Transformation|GetActorLocation) "0, 0, 0" 1.0 1.0 0.0 0 0 0))))

(event EventStop
  (CallFunction|StopFire))

(event EventCleanChamber
  (CallFunction|ClearChamber))

(event EventPopUp
  (params (Character :type Top%20Down%20Character%20Object%20Reference))
  (Default|PopUp (Variables|Default|GetBP_WidgetComponent) Character))

(fn ConstructionScript)

(fn StartFire
  (bind _skeletalmesh (Variables|Default|GetSkeletalMesh))
  (bind _currentbullet (Variables|Default|GetCurrentBullet))
  (bind _returnvalue (Transformation|GetSocketTransform _skeletalmesh "MuzzleSocket" "RTS_World"))
  (if (Variables|Default|GetbIsJammed)
    (Development|PrintString "Chamber Jammed")
    (else
      (Development|PrintString "Shot")
      (if (Variables|Default|GetbIsChamberLoaded)
        (Game|SpawnActorfromClass "/Game/Blueprints/BP_Bullet.BP_Bullet_C" (Math|Transform|MakeTransform (.location _returnvalue) (.rotation _returnvalue) "3.000000,3.000000,3.000000") "Undefined" 0 (Variables|/Script/Pathogenesis.Ammo|GetAmmoDamage _currentbullet) (Variables|/Script/Pathogenesis.Ammo|GetAmmoMesh _currentbullet) (Variables|/Script/Pathogenesis.Ammo|GetPenetration _currentbullet) 0)
        (Audio|SpawnSoundatLocation "/Game/Audio/Rifle_Cue.Rifle_Cue" (.location _returnvalue) "0, 0, 0" 1.0 1.0 0.0 0 0)
        (CallFunction|ChamberReload)
        (else
          (Audio|PlaySoundatLocation "/Game/Audio/TriggerClick.TriggerClick" (Transformation|GetActorLocation) "0, 0, 0" 1.0 1.0 0.0 0 0 0))))))

(fn ChamberReload
  (Audio|PlaySoundatLocation "/Game/Audio/ChamberReload.ChamberReload" (Transformation|GetActorLocation) "0, 0, 0" 0.5 1.5 0.0 0 0 0)
  (if (Variables|Default|GetbIsChamberLoaded)
    (bind _shell_dropped (CallFunction|DropShell))
    (if _shell_dropped
      (Variables|Default|SetbIsChamberLoaded false)
      (Class|WeaponActor|LoadBullet)
      (else
        (Development|PrintString "Chamber Jammed")))
    (else
      (Class|WeaponActor|LoadBullet))))

(fn StopFire
  (Utilities|Time|ClearandInvalidateTimerbyHandle (Variables|Default|GetFireHandle)))

(fn DropShell
  (bind _skeletalmesh (Variables|Default|GetSkeletalMesh))
  (bind _returnvalue (Transformation|GetSocketTransform _skeletalmesh "ChamberSocket" "RTS_World"))
  (if (> (Math|Random|RandomFloatinRange 0.0 1e+02) 99.0)
    (Variables|Default|SetbIsJammed true)
    (Development|PrintString "Chamber Jammed")
    (return false)
    (else
      (Game|SpawnActorfromClass "/Game/Blueprints/BP_BulletShell.BP_BulletShell_C" (Math|Transform|MakeTransform (.location _returnvalue) (.rotation _returnvalue) "3.000000,3.000000,3.000000") "Undefined" 0 0)
      (return true))))

(fn ClearChamber
  (bind _skeletalmesh (Variables|Default|GetSkeletalMesh))
  (bind _returnvalue (Transformation|GetSocketTransform _skeletalmesh "ChamberSocket" "RTS_World"))
  (Audio|PlaySoundatLocation "/Game/Audio/ChamberReload.ChamberReload" (Transformation|GetActorLocation) "0, 0, 0" 0.5 1.5 0.0 0 0 0)
  (if (Variables|Default|GetbIsChamberLoaded)
    (Variables|Default|SetbIsJammed false)
    (Game|SpawnActorfromClass "/Game/Blueprints/BP_BulletShell.BP_BulletShell_C" (Math|Transform|MakeTransform (.location _returnvalue) (.rotation _returnvalue) "3.000000,3.000000,3.000000") "Undefined" 0 0))
  (Class|WeaponActor|LoadBullet))

(fn Initialize
  (bind _itemdata (Variables|Default|GetItemData))
  (bind _asweapon (Utilities|Casting|CastToWeapon _itemdata))
  (Variables|Default|SetAmmoType (Variables|/Script/Pathogenesis.Weapon|GetAmmoType _asweapon))
  (Variables|Default|SetFireRate (Variables|/Script/Pathogenesis.Weapon|GetFireRate _asweapon))
  (Variables|Default|SetbIsFullAuto (Variables|/Script/Pathogenesis.Weapon|GetbIsFullAuto _asweapon))
  (Variables|Default|SetCount (Variables|/Script/Pathogenesis.Item|GetCount _asweapon))
  (Class|SkinnedMeshComponent|SetSkeletalMesh (Variables|Default|GetSkeletalMesh) (Variables|/Script/Pathogenesis.Weapon|GetWeaponMesh _asweapon) false)
  (Variables|/Game/Blueprints/Components/BP_WidgetComponent.BP_WidgetComponent_C|SetName (Variables|Default|GetBP_WidgetComponent) (Variables|/Script/Pathogenesis.Item|GetItemName (Variables|Default|GetItemData))))