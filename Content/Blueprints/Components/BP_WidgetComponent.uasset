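; BP_WidgetComponent is a widget component that shows and hides an interaction pop-up for a character.
; The PopUp event displays the component's Name text on its WBP_InteractionPopUp widget and binds hiding to the character's OnPopUpChanged dispatcher.
; When that dispatcher fires, the widget collapses.
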(event Custom|HidPopUp
  (CallFunction|HidePopUp))

(event EventPopUp
  (params (Character :type Top%20Down%20Character%20Object%20Reference))
  (CallFunction|ShowPopUp (Variables|Default|GetName))
  (EventDispatchers|BindEventtoOnPopUpChanged Character (delegate Custom|HidPopUp)))

(fn ShowPopUp
  (params (Text :type Text))
  (bind _aswbp_interaction_pop_up (Utilities|Casting|CastToWBP_InteractionPopUp (UserInterface|GetWidget)))
  (Rendering|Components|TextRender|SetText (Variables|/Game/UI/Inventory/WBP_InteractionPopUp.WBP_InteractionPopUp_C|GetPopUpText _aswbp_interaction_pop_up) Text)
  (Widget|SetVisibility _aswbp_interaction_pop_up "SelfHitTestInvisible"))

(fn HidePopUp
  (bind _aswbp_interaction_pop_up (Utilities|Casting|CastToWBP_InteractionPopUp (UserInterface|GetWidget)))
  (Widget|SetVisibility _aswbp_interaction_pop_up "Collapsed"))