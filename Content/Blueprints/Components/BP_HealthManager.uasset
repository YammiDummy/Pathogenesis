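; BP_HealthManager is a health component that tracks current health against a maximum.
; TakeDamage subtracts damage only while health is above zero, clamping the result at zero.
; Each hit broadcasts OnDamageTaken with the health fraction from GetHealthPercentage, and the lethal hit also broadcasts OnDeath.
; The event graph is unused, so all logic runs through function calls and event dispatchers.
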(event EventBeginPlay)

(event EventTick
  (params (DeltaSeconds :type Float%20%28single-precision%29)))

(fn TakeDamage
  (params (Damage :type Float%20%28single-precision%29))
  (if (> (Variables|Default|GetCurrentHealth) 0.0)
    (if (> (- (Variables|Default|GetCurrentHealth) Damage) 0.0)
      (Variables|Default|SetCurrentHealth (- (Variables|Default|GetCurrentHealth) Damage))
      (Default|CallOnDamageTaken (CallFunction|GetHealthPercentage))
      (else
        (Variables|Default|SetCurrentHealth 0.0)
        (Default|CallOnDamageTaken (CallFunction|GetHealthPercentage))
        (Default|CallOnDeath)))))

(fn GetHealthPercentage
  (return (/ (Variables|Default|GetCurrentHealth) (Variables|Default|GetMaximumHealth))))