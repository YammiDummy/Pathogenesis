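; Bullet projectile actor that damages targets, penetrates walls and plays surface-based impact effects.
; Overlapping a BP_Wall plays a concrete or wood sound, adds a decal, then subtracts wall thickness from Penetration or destroys the bullet if too thick.
; Blocking hits send damage through BPI_Damage, boosted for "Head" bone hits, or spawn surface sound and decal on other objects, then destroy the bullet.
; The construction script applies the configured bullet mesh.
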(event OnComponentHit(BulletMeshComponent)
  (params (HitComponent :type Primitive%20Component%20Object%20Reference) (OtherActor :type Actor%20Object%20Reference) (OtherComp :type Primitive%20Component%20Object%20Reference) (NormalImpulse :type Vector :default "0, 0, 0") (Hit :type Hit%20Result%20Structure%20%28by%20ref%29))
  (bind (_bblockinghit _binitialoverlap _time _distance _location _impactpoint _normal _impactnormal _physmat _hitactor _hitcomponent) (Collision|BreakHitResult Hit))
  (bind (_bblockinghit_2 _binitialoverlap_2 _time_2 _distance_2 _location_2 _impactpoint_2 _normal_2 _impactnormal_2 _physmat_2 _hitactor_2 _hitcomponent_2 _hitbonename) (Collision|BreakHitResult Hit))
  (bind _damage (Variables|Default|GetDamage))
  (Development|PrintString (Utilities|GetDisplayName OtherComp))
  (if (Utilities|DoesObjectImplementInterface OtherActor "/Game/Interfaces/BPI_Damage.BPI_Damage_C")
    (Class|BPIDamage|TakeDamage(Message) OtherActor (Math|Float|SelectFloat (* _damage 1.5) _damage (Utilities|Name|Equal(Name) _hitbonename "Head")))
    (Audio|PlaySoundatLocation "/Game/Audio/Hit_Flesh_Cue.Hit_Flesh_Cue" _impactpoint_2 "0, 0, 0" 1.0 1.0 0.0 0 0 0)
    (Actor|DestroyActor)
    (else
      (switch Utilities|FlowControl|Switch|SwitchonEPhysicalSurface (Variables|/Script/PhysicsCore.PhysicalMaterial|GetSurfaceType _physmat)
        (:SurfaceType_Default
          (Audio|PlaySoundatLocation "/Game/Audio/Hit_Concrete_Cue.Hit_Concrete_Cue" _impactpoint "0, 0, 0" 1.0 1.0 0.0 0 0 0 :!label _label))
        (:SurfaceType1
          (goto _label))
        (:SurfaceType2
          (Audio|PlaySoundatLocation "/Game/Audio/Hit_Wood_Cue.Hit_Wood_Cue" _impactpoint "0, 0, 0" 1.0 1.0 0.0 0 0 0))
        (:SurfaceType3
          (Audio|PlaySoundatLocation "/Game/Audio/Hit_Flesh_Cue.Hit_Flesh_Cue" _impactpoint "0, 0, 0" 1.0 1.0 0.0 0 0 0)))
      (Class|GameplayStatics|SpawnDecalAttached "/Game/Textures/Hit_Decal_Mat.Hit_Decal_Mat" "20.000000,20.000000,20.000000" _hitcomponent "None" _impactpoint (Math|Rotator|MakeRotfromX _impactnormal) "KeepWorldPosition" 1e+01)
      (Actor|DestroyActor))))

(event OnComponentBeginOverlap(BulletMeshComponent)
  (params (OverlappedComponent :type Primitive%20Component%20Object%20Reference) (OtherActor :type Actor%20Object%20Reference) (OtherComp :type Primitive%20Component%20Object%20Reference) (OtherBodyIndex :type Integer) (bFromSweep :type Boolean) (SweepResult :type Hit%20Result%20Structure%20%28by%20ref%29))
  (bind (_bblockinghit _binitialoverlap _time _distance _location _impactpoint _normal _impactnormal _physmat _hitactor _hitcomponent) (Collision|BreakHitResult SweepResult))
  (Development|PrintString (Utilities|GetDisplayName OtherComp))
  (bind _asbp_wall (Utilities|Casting|CastToBP_Wall OtherActor))
  (switch Utilities|FlowControl|Switch|SwitchonEPhysicalSurface (Variables|/Script/PhysicsCore.PhysicalMaterial|GetSurfaceType _physmat)
    (:SurfaceType1
      (Audio|PlaySoundatLocation "/Game/Audio/Hit_Concrete_Cue.Hit_Concrete_Cue" "0, 0, 0" "0, 0, 0" 1.0 1.0 0.0 0 0 0))
    (:SurfaceType2
      (Audio|PlaySoundatLocation "/Game/Audio/Hit_Wood_Cue.Hit_Wood_Cue" "0, 0, 0" "0, 0, 0" 1.0 1.0 0.0 0 0 0)))
  (Class|GameplayStatics|SpawnDecalAttached "/Game/Textures/Hit_Decal_Mat.Hit_Decal_Mat" "20.000000,20.000000,20.000000" _hitcomponent "None" _impactpoint (Math|Rotator|MakeRotfromX _impactnormal) "KeepWorldPosition" 1e+01)
  (if (> (Variables|/Game/Blueprints/BP_Wall.BP_Wall_C|GetThickness _asbp_wall) (Variables|Default|GetPenetration))
    (Actor|DestroyActor)
    (else
      (Variables|Default|SetPenetration (- (Variables|Default|GetPenetration) (Variables|/Game/Blueprints/BP_Wall.BP_Wall_C|GetThickness _asbp_wall))))))

(fn ConstructionScript
  (Components|StaticMesh|SetStaticMesh (Variables|Default|GetBulletMeshComponent) (Variables|Default|GetBulletMesh)))

(fn Initialize)