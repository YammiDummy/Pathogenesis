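; BP_AmmoMaster is the base ammo pickup that characters can pick up.
; PopUp forwards to the widget component to show a prompt for the character, and Interact passes the item to the character's PickUpItem.
; The construction script names the widget from ItemData, then casts it to Ammo to set the ammo type, count and mesh material, so each pickup is data-driven.
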(event EventPopUp
  (params (Character :type Top%20Down%20Character%20Object%20Reference))
  (Default|PopUp (Variables|Default|GetBP_WidgetComponent) Character))

(event EventInteract
  (params (Character :type Top%20Down%20Character%20Object%20Reference))
  (Class|PathogenesisCharacter|PickUpItem Character self))

(fn ConstructionScript
  (bind _itemdata (Variables|Default|GetItemData))
  (Variables|/Game/Blueprints/Components/BP_WidgetComponent.BP_WidgetComponent_C|SetName (Variables|Default|GetBP_WidgetComponent) (Variables|/Script/Pathogenesis.Item|GetItemName (Variables|Default|GetItemData)))
  (bind _asammo (Utilities|Casting|CastToAmmo _itemdata))
  (Variables|Default|SetAmmoType (Variables|/Script/Pathogenesis.Ammo|GetAmmoType _asammo))
  (Variables|Default|SetCount (Variables|/Script/Pathogenesis.Item|GetCount _itemdata))
  (Rendering|Material|SetMaterial (Variables|Default|GetStaticMesh) 0 (Variables|/Script/Pathogenesis.Ammo|GetAmmoMaterial _asammo)))