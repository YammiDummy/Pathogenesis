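; BP_MedKit is a med kit item actor configured from a Supplies data object.
; Its construction script casts ItemData to Supplies, copies Count and Power, sets the mesh and passes the item name to its widget component.
; A PopUp event forwards the given character to that widget component, while BeginPlay, overlap and Tick are unused.
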(event EventBeginPlay)

(event Collision|EventActorBeginOverlap
  (params (OtherActor :type Actor%20Object%20Reference)))

(event EventTick
  (params (DeltaSeconds :type Float%20%28single-precision%29)))

(event EventPopUp
  (params (Character :type Top%20Down%20Character%20Object%20Reference))
  (Default|PopUp (Variables|Default|GetBP_WidgetComponent) Character))

(fn ConstructionScript
  (bind _assupplies (Utilities|Casting|CastToSupplies (Variables|Default|GetItemData)))
  (Variables|Default|SetCount (Variables|/Script/Pathogenesis.Item|GetCount _assupplies))
  (Variables|Default|SetPower (Variables|/Script/Pathogenesis.Supplies|GetPower _assupplies))
  (Components|StaticMesh|SetStaticMesh (Variables|Default|GetMedKitMesh) (Variables|/Script/Pathogenesis.Supplies|GetSupplyMesh _assupplies))
  (Variables|/Game/Blueprints/Components/BP_WidgetComponent.BP_WidgetComponent_C|SetName (Variables|Default|GetBP_WidgetComponent) (Variables|/Script/Pathogenesis.Item|GetItemName _assupplies)))